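; Ludwig Junior is the tutorial NPC who talks Coots through movement, attacking a Dummy and parrying, using timed lines in the DIALOUGE widget.
; BeginPlay runs the intro and sets up the Dummy; Nextline starts the parry lesson and spawns a SwordCrow.
; Tick respawns dead crows until Counter reaches three, then saves tutorial completion.
; A timeline-driven material dissolve removes his mesh on completion or when the save already records it.
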(event `self.ReceiveBeginPlay`
  (bind _array (`|MakeArray` "GOOD MORNING COOTS!" "THE CROWS ARE INVADING OUR LAND AND YOU HAVE TO GET READY!" "START BY STRECH YOUR LEGS ABIT USING W,A,S,D ,LEFT SHIFT AND SPACE TO DASH" "GOOD... NOW KILL THAT DUMMY OVER THERE WITH YOUR SECRET SWORD TECHNIC *LEFT MOUSE*"))
  (bind _returnvalue (`GameplayStatics.LoadGameFromSlot` "1"))
  (bind _assave_game_1 (cast `/Game/saveGame1` _returnvalue))
  (if (>= (`/Game/saveGame1.Tutorial` _assave_game_1) 1)
    (`self.Disslove`))
  (bind _asdialouge (cast `/Game/ThirdPersonBP/Blueprints/DIALOUGE` (`WidgetComponent.GetWidget` (`self.Widget`))))
  (bind _output_get (set `self.As DIALOUGE` _asdialouge))
  (`/Game/ThirdPersonBP/Blueprints/DIALOUGE.SetPic` _asdialouge "/Game/ThirdPersonBP/Blueprints/LudwigJuniorshead.LudwigJuniorshead")
  (set `/Game/ThirdPersonBP/Blueprints/DIALOUGE.Dialouges` _array _output_get)
  (`/Game/ThirdPersonBP/Blueprints/DIALOUGE.Talk` _output_get false :!label _label)
  (`KismetSystemLibrary.Delay` 5.0)
  (if (< (`self.Repeat`) (`KismetArrayLibrary.Array_Length` _array))
    (`/Engine/EditorBlueprintResources/StandardMacros.IncrementInt` (`self.Repeat`)
      (:`  `
        (goto _label)))
    (else
      (bind _returnvalue_2 (`GameplayStatics.GetActorOfClass` "/Game/Enemies/Dummy.Dummy_C"))
      (bind _output_get_2 (set `/Game/Enemies/Dummy.Max_Hp` 10.0 _returnvalue_2))
      (set `/Game/Enemies/Dummy.Hp` _output_get_2 _returnvalue_2)
      (set `/Game/Enemies/Dummy.DmgRd` 1.0 _returnvalue_2))))

(event `Nextline`
  (bind _as_dialouge (`self.As DIALOUGE`))
  (bind _as_dialouge_2 (`self.As DIALOUGE`))
  (set `/Game/ThirdPersonBP/Blueprints/DIALOUGE.Dialouges` (`|MakeArray` "GOOOD... COOTS! HERE ONE OF THEM COMES" "YOU CAN PARRY NORMAL ATTACKS AND PROJECTILES WITH \"Q\"" "TRY TOO PARRY 3 TIMES") _as_dialouge)
  (set `/Game/ThirdPersonBP/Blueprints/DIALOUGE.CurrentLine` 0 _as_dialouge)
  (set `/Game/ThirdPersonBP/Blueprints/DIALOUGE.ActiveText` "" _as_dialouge)
  (`/Game/ThirdPersonBP/Blueprints/DIALOUGE.Talk` _as_dialouge false)
  (`KismetSystemLibrary.Delay` 5.0)
  (bind _returnvalue (`GameplayStatics.GetActorOfClass` "/Game/ThirdPersonBP/Blueprints/Coots.Coots_C"))
  (set `/Game/ThirdPersonBP/Blueprints/Coots.TutorialActive` true _returnvalue)
  (`/Game/ThirdPersonBP/Blueprints/HUD.ParryTut` (`/Game/ThirdPersonBP/Blueprints/Coots.Hud` _returnvalue))
  (`/Game/ThirdPersonBP/Blueprints/DIALOUGE.Talk` (`self.As DIALOUGE`) false)
  (`KismetSystemLibrary.Delay` 5.0)
  (`/Game/ThirdPersonBP/Blueprints/DIALOUGE.Talk` (`self.As DIALOUGE`) false)
  (`KismetSystemLibrary.Delay` 5.0)
  (set `/Game/ThirdPersonBP/Blueprints/DIALOUGE.Dialouges` (`|MakeArray` "1!! 2 MORE TO GO" "2!! 1 MORE TO GO" "WELL DONE COOTS. NOW FINISH  HIM OFF!") _as_dialouge_2)
  (set `/Game/ThirdPersonBP/Blueprints/DIALOUGE.CurrentLine` 0 _as_dialouge_2)
  (set `/Game/ThirdPersonBP/Blueprints/DIALOUGE.ActiveText` "" _as_dialouge_2)
  (bind _returnvalue_2 (`|SpawnActorFromClass` "/Game/Enemies/SwordCrow.SwordCrow_C" (`KismetMathLibrary.MakeTransform` (-1230.0 1430.0 180.0)) "Undefined" "OverrideRootScale" null null))
  (bind _output_get (set `self.CurrentCrow` _returnvalue_2))
  (`self.SetActorTickEnabled` true)
  (`self.SetActorTickEnabled` _output_get true))

(event `self.ReceiveTick`
  (params (DeltaSeconds :type "Float (single-precision)"))
  (bind _as_dialouge (`self.As DIALOUGE`))
  (if (< (`/Game/Enemies/BaseEnemy.Hp` (`self.CurrentCrow`)) 1.0)
    (if (< (`self.Counter`) 3)
      (bind _returnvalue (`|SpawnActorFromClass` "/Game/Enemies/SwordCrow.SwordCrow_C" (`KismetMathLibrary.MakeTransform` (-1230.0 1430.0 180.0)) "Undefined" "OverrideRootScale" null null))
      (bind _output_get (set `self.CurrentCrow` _returnvalue))
      (`self.SetActorTickEnabled` _output_get true)
      (else
        (bind _returnvalue_2 (`GameplayStatics.GetActorOfClass` "/Game/ThirdPersonBP/Blueprints/Coots.Coots_C"))
        (set `/Game/ThirdPersonBP/Blueprints/Coots.TutorialActive` false _returnvalue_2)
        (`self.SetActorTickEnabled` false)
        (set `/Game/ThirdPersonBP/Blueprints/DIALOUGE.Dialouges` (`|MakeArray` "NOW GO AND FREE OUR LAND FROM THESE WICKED CROWS") _as_dialouge)
        (set `/Game/ThirdPersonBP/Blueprints/DIALOUGE.CurrentLine` 0 _as_dialouge)
        (set `/Game/ThirdPersonBP/Blueprints/DIALOUGE.ActiveText` "" _as_dialouge)
        (set `/Game/ThirdPersonBP/Blueprints/DIALOUGE.Index` 0 _as_dialouge)
        (`/Game/ThirdPersonBP/Blueprints/DIALOUGE.Talk` _as_dialouge false)
        (`self.SetActorTickEnabled` false)
        (`self.Disslove`)
        (`KismetSystemLibrary.Delay` 3.0)
        (bind _returnvalue_3 (`GameplayStatics.GetActorOfClass` "/Game/ThirdPersonBP/Blueprints/Coots.Coots_C"))
        (`/Game/ThirdPersonBP/Blueprints/Coots.ByeDers` _returnvalue_3)
        (bind _returnvalue_4 (`GameplayStatics.LoadGameFromSlot` "1"))
        (bind _assave_game_1 (cast `/Game/saveGame1` _returnvalue_4))
        (bind _output_get_2 (set `/Game/saveGame1.Tutorial` 1 _assave_game_1))
        (set `/Game/ThirdPersonBP/Blueprints/Coots.Tutorials` _output_get_2 _returnvalue_3)
        (`GameplayStatics.SaveGameToSlot` _assave_game_1 "1")))))

(event `ParryTutorial`
  (`/Game/ThirdPersonBP/Blueprints/DIALOUGE.Talk` (`self.As DIALOUGE`) false))

(event `Disslove`
  (bind (_direction _newtrack_0) (`Timeline|Timeline_0` :!via `PlayFromStart`)
    (:`Update`
      (`MaterialInstanceDynamic.SetScalarParameterValue` (`self.Mat`) "Disslove" _newtrack_0))
    (:`Finished`
      (`ActorComponent.K2_DestroyComponent` (`self.StaticMesh1`)))))

(fn `UserConstructionScript`
  (bind _staticmesh1 (`self.StaticMesh1`))
  (bind _returnvalue (`PrimitiveComponent.CreateDynamicMaterialInstance` _staticmesh1 0 (`PrimitiveComponent.GetMaterial` _staticmesh1 0) "None"))
  (set `self.Mat` _returnvalue))